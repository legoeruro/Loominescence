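; Small enemy mob that loops through waypoints via AI MoveTo, can chase the player, and damages them on capsule contact.
; Potion events apply float, double attack (knock-up on hit), speed, heal or explosion effects, with colored Niagara FX spawned during lasting effects.
; Tick drives frame-based cooldowns, effect expiry, the health bar and death, which drops an item and requests a respawn when a drop class is set.
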(event `self.ReceiveTick`
  (params (DeltaSeconds :type "Float (single-precision)"))
  (bind (_returnvalue_location _returnvalue_rotation) (`KismetMathLibrary.BreakTransform` (`self.GetTransform`)))
  (bind _itemdropclass (`self.ItemDropClass`))
  ; Event Tick
  (`|ExecutionSequence`
    (:`then_0`
      ;; Countdown
      (set `self.Attack Countdown` (`KismetMathLibrary.Clamp` (- (`self.Attack Countdown`) 1) 0 100))
      (set `self.DoubleAttack CountDown` (`KismetMathLibrary.Clamp` (- (`self.DoubleAttack CountDown`) 1) 0 100))
      (set `self.FloatCountDown` (`KismetMathLibrary.Clamp` (- (`self.FloatCountDown`) 1) 0 100))
      (`|ExecutionSequence`
        (:`then_0`
          ; Each Effect CountDown
          (if (`self.IsDoubleAttack`)
            (if (== 0 (`self.DoubleAttack CountDown`))
              (set `self.IsDoubleAttack` false)
              (set `self.InEffect?` false))))
        (:`then_1`
          (if (`self.IsFloat`)
            (if (== (`self.FloatCountDown`) 0)
              (`self.LaunchCharacter` (`KismetMathLibrary.MakeVector` 0.0 0.0 (`self.RiseSpeed`)))
              (set `self.InEffect?` false)
              (set `self.IsFloat` false)
              (`self.Follow Waypoints`))))))
    (:`then_1`
      ;; Add Particle Effect
      (switch `string` (`self.PotionType`)
        (:`Float`
          (set `self.PotionColorFX` (struct :`G` 1.0 :`B` 0.481061 :`A` 1.0)))
        (:`DoubleAttack`
          (set `self.PotionColorFX` (struct :`R` 1.0 :`G` 0.959396 :`B` 0.236419 :`A` 1.0)))
        (:`Speed`
          (set `self.PotionColorFX` (struct :`R` 0.005181 :`G` 0.010356 :`B` 0.333333 :`A` 1.0)))
        (:`Heal`
          (set `self.PotionColorFX` (struct :`R` 0.175261 :`G` 1.0 :`A` 1.0)))))
    (:`then_2`
      (if (`self.InEffect?`)
        (bind _returnvalue (`NiagaraFunctionLibrary.SpawnSystemAtLocation` "/Game/Assets/ParticalEffect/NS_EnemyPotionEffect.NS_EnemyPotionEffect" _returnvalue_location _returnvalue_rotation))
        (`NiagaraComponent.SetVariableLinearColor` _returnvalue "PotionColor" (`self.PotionColorFX`))))
    (:`then_3`
      ;; Health
      (if (== (`self.Health`) 0.0)
        ;; After death, drop item
        (if (`KismetSystemLibrary.IsValidClass` _itemdropclass)
          (`|SpawnActorFromClass` _itemdropclass (`self.GetTransform`) "Undefined" "MultiplyWithRoot" null null)
          (`/Game/Blueprints/Enemies/BP_EnemySpanwer.Request Respawn` (`self.Spawner`) (`self.GetTransform`))
          (`self.K2_DestroyActor`))
        (else
          (bind _aswbp_health_bar (cast `/Game/Blueprints/Enemies/WBP_HealthBar` (`WidgetComponent.GetWidget` (`self.HealthBar Widget`))))
          (`ProgressBar.SetPercent` (`/Game/Blueprints/Enemies/WBP_HealthBar.HealthBar` _aswbp_health_bar) (/ (`self.Health`) 100.0)))))))

(event `self.ReceiveBeginPlay`
  (`self.Follow Waypoints`))

(event `Chase Player`
  (`|AIMoveTo` self (0.0 0.0 0.0) (`GameplayStatics.GetPlayerCharacter` 0)))

(event `self.ReceiveAnyDamage`
  (params (Damage :type "Float (single-precision)") (DamageType :type "DamageType Object Reference") (InstigatedBy :type "Controller Object Reference") (DamageCauser :type "Actor Object Reference"))
  (bind _returnvalue (- (`self.Health`) Damage))
  ; Event Tick
  ;; Health
  (if (> _returnvalue 0.0)
    (set `self.Health` _returnvalue)
    (else
      (set `self.Health` 0.0)
      (set `self.IsDead` true))))

(event `self.CapsuleComponent.OnComponentHit`
  (params (HitComponent :type "PrimitiveComponent Object Reference") (OtherActor :type "Actor Object Reference") (OtherComp :type "PrimitiveComponent Object Reference") (NormalImpulse :type "Vector Structure") (Hit :type "HitResult Structure (by ref)"))
  ; Attack / Deal Damage
  (if (== (`self.Attack Countdown`) 0)
    (if (!= OtherActor self)
      (bind _asbp_player_base (cast `/Game/Blueprints/Player/BP_PlayerBase` OtherActor))
      (`GameplayStatics.ApplyDamage` _asbp_player_base 10.0)
      (set `self.Attack Countdown` 50)
      (if (`self.IsDoubleAttack`)
        (`self.LaunchCharacter` _asbp_player_base (0.0 0.0 1000.0) false false)))))

(event `Follow Waypoints`
  ; Follow Waypoints
  (`|AIMoveTo` self (0.0 0.0 0.0) (`|GetArrayItem` (`self.Waypoint`) (`self.Current Waypoint`))
    (:`OnSuccess`
      (`/Engine/EditorBlueprintResources/StandardMacros.IncrementInt` (`self.Current Waypoint`)
        (:`  `
          (if (>= (`self.Current Waypoint`) (`KismetArrayLibrary.Array_Length` (`self.Waypoint`)))
            (set `self.Current Waypoint` 0)
            (`self.Follow Waypoints`)
            (else
              (`self.Follow Waypoints`))))))))

(event `FloatUp`
  (bind _charactermovement (`self.CharacterMovement`))
  ; Float Up
  (set `self.PotionType` "Float")
  (set `self.IsFloat` true)
  (set `self.InEffect?` true)
  (`MovementComponent.StopMovementImmediately` _charactermovement)
  (set `CharacterMovementComponent.GravityScale` 0.0 _charactermovement)
  (`self.LaunchCharacter` (0.0 0.0 40.0))
  (set `self.FloatCountDown` 500))

(event `DoubleAttack`
  ; Double Attack
  (set `self.PotionType` "DoubleAttack")
  (set `self.InEffect?` true)
  (set `self.IsDoubleAttack` true)
  (set `self.DoubleAttack CountDown` 2000))

(event `Explode`
  (bind (_returnvalue_location _returnvalue_rotation) (`KismetMathLibrary.BreakTransform` (`self.GetTransform`)))
  ; Explosion
  (set `self.Health` (`KismetMathLibrary.FClamp` (- (`self.Health`) 70.0) 0.0 (`self.Max Health`)))
  (`NiagaraFunctionLibrary.SpawnSystemAtLocation` "/Game/Assets/ParticalEffect/NS_Explosion.NS_Explosion" _returnvalue_location _returnvalue_rotation))

(event `Increase Speed`
  (bind _charactermovement (`self.CharacterMovement`))
  ; Increase Speed
  (set `self.PotionType` "Speed")
  (set `self.InEffect?` true)
  (set `CharacterMovementComponent.MaxWalkSpeed` (* (`CharacterMovementComponent.MaxWalkSpeed` _charactermovement) 2.0) _charactermovement)
  (`KismetSystemLibrary.Delay` 5.0)
  (set `CharacterMovementComponent.MaxWalkSpeed` (`self.Max Walk Speed Default`) (`self.CharacterMovement`))
  (set `self.InEffect?` false))

(event `Heal`
  ; Heal
  (set `self.PotionType` "Heal")
  (set `self.InEffect?` true)
  (for _ (range 5)
    (set `self.Health` (`KismetMathLibrary.FClamp` (+ (`self.Health`) 5.0) 0.0 (`self.Max Health`))))
  (set `self.InEffect?` false))

(fn `Attack`
  (params (Target :type "/Game/Blueprints/Player/BP_PlayerBase Object Reference") (Damage :type "Float (double-precision)"))
  (`GameplayStatics.ApplyDamage` Target Damage))

(fn `UserConstructionScript`)