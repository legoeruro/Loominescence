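; BP_VineDoor is a door actor that shows a widget while something overlaps its Box and moves toward an open location when its Craft event fires.
; Craft runs a LoopWithDelay macro, stepping the actor toward OpenLocation with VInterpTo, using DelayTime as both loop delay and interpolation delta.
; The motion runs for a fixed iteration count without Tick or Timeline, so it eases out and may stop short of the target.
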(event `self.Box.OnComponentBeginOverlap`
  (params (OverlappedComponent :type "PrimitiveComponent Object Reference") (OtherActor :type "Actor Object Reference") (OtherComp :type "PrimitiveComponent Object Reference") (OtherBodyIndex :type Integer) (bFromSweep :type Boolean) (SweepResult :type "HitResult Structure (by ref)"))
  (`SceneComponent.SetVisibility` (`self.Widget`) true false))

(event `self.Box.OnComponentEndOverlap`
  (params (OverlappedComponent :type "PrimitiveComponent Object Reference") (OtherActor :type "Actor Object Reference") (OtherComp :type "PrimitiveComponent Object Reference") (OtherBodyIndex :type Integer))
  (`SceneComponent.SetVisibility` (`self.Widget`) false false))

(event `/Game/Blueprints/Potion/BPI_Crafting.Craft`
  (bind _delay_time (`self.Delay Time`))
  (`self.LoopWithDelay` 0 20 _delay_time
    (:`Loop Body`
      (`self.K2_SetActorLocation` (`KismetMathLibrary.VInterpTo` (`self.K2_GetActorLocation`) (`self.OpenLocation`) _delay_time 1.0)))))

(fn `UserConstructionScript`)