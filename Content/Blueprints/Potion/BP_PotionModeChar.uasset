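; BP_PotionModeChar is an unfinished character for the potion mode, meant to move a hand and grab through Enhanced Input.
; On BeginPlay it adds the potion mapping context to its player controller.
; The move action feeds control-rotation movement input, then clamps the capsule's X and Y to a 1920x1080 range, but both calls are marked disabled.
; Grab is a todo with a disabled test print.
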(event `self.ReceiveBeginPlay`
  ; remove?
  (bind _asplayer_controller (cast `PlayerController` (`self.GetController`)))
  (`EnhancedInputSubsystemInterface.AddMappingContext` (pcsubsystem `EnhancedInputLocalPlayerSubsystem` _asplayer_controller) "/Game/InputAction/PotionSystem/IMC_PotionSystem.IMC_PotionSystem" 0 (struct)))

(fn `ClampLocation`
  (bind (_returnvalue_x _returnvalue_y _returnvalue_z) (`KismetMathLibrary.BreakVector` (`SceneComponent.K2_GetComponentLocation` (`self.CapsuleComponent`))))
  (`SceneComponent.K2_SetWorldLocation` (`self.CapsuleComponent`) (`KismetMathLibrary.MakeVector` (`KismetMathLibrary.FClamp` _returnvalue_x 0.0 1920.0) (`KismetMathLibrary.FClamp` _returnvalue_y 0.0 1080.0) _returnvalue_z) false false))

(fn `Move`
  (params (`X Axis` :type "Float (double-precision)") (`Y Axis` :type "Float (double-precision)"))
  ; x axis
  (`self.AddMovementInput` (`KismetMathLibrary.GetForwardVector` (`self.GetControlRotation`)) `X Axis`)
  ; y axis
  (`self.AddMovementInput` (`KismetMathLibrary.GetRightVector` (`self.GetControlRotation`)) `Y Axis`))

(fn `UserConstructionScript`)