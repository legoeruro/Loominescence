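; Cauldron Blueprint for potion crafting that supplies a tooltip describing itself and the ingredients it consists of.
; GetTooltipData joins a rich-text title, a description and the string from GetStringListOfIngredients, then returns the result as TooltipData.
; The event graph and construction script are empty, so the tooltip is the only logic defined here.
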(fn `GetTooltipData`
  (returns (ReturnValue :type "TooltipData Structure"))
  (locals (`Strings to print tooltip` :type "Array of String"))
  (bind _strings_to_print_tooltip (`local.Strings to print tooltip`))
  (`KismetArrayLibrary.Array_Add` _strings_to_print_tooltip "<Title> Cauldron  </> \n")
  (`KismetArrayLibrary.Array_Add` _strings_to_print_tooltip "<Description> A cauldron consisting of several ingredients: </> \n<Description> ")
  (`KismetArrayLibrary.Array_Add` _strings_to_print_tooltip (`self.GetStringListOfIngredients`))
  (`KismetArrayLibrary.Array_Add` (`local.Strings to print tooltip`) "</>")
  (return (make `TooltipData` (`KismetStringLibrary.JoinStringArray` (`local.Strings to print tooltip`) ""))))

(fn `UserConstructionScript`)