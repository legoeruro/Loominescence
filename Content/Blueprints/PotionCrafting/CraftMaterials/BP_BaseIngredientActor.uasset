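; Base actor for a potion-crafting ingredient, carrying an item struct (ThisItem) that links it to the player's inventory.
; CleanuponDestroy uses the player's BPC_InventoryMiniComponent to remove one held item if it was used, or add it back to inventory otherwise, then prints debug strings.
; GetTooltipData joins the item's name and description with rich-text style tags into tooltip data.
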(event `self.CleanupOnDestroy`
  (params (WasItemUsed :type Boolean))
  (bind _this_item (`self.This Item`))
  (bind _returnvalue (`self.GetComponentByClass` (`GameplayStatics.GetPlayerCharacter` 0) "/Game/Inventory/BPC_InventoryMiniComponent.BPC_InventoryMiniComponent_C"))
  (if WasItemUsed
    (`/Game/Inventory/BPC_InventoryMiniComponent.Remove One Item From ItemsToHold` _returnvalue _this_item)
    (else
      (`/Game/Inventory/BPC_InventoryMiniComponent.Add to Inventory with Item Struct` _returnvalue _this_item)))
  (`KismetSystemLibrary.PrintString` "cleanup")
  (`KismetSystemLibrary.PrintString` (`KismetStringLibrary.Conv_BoolToString` WasItemUsed)))

(fn `GetTooltipData`
  (returns (ReturnValue :type "TooltipData Structure"))
  (locals (`Tooltip List` :type "Array of String"))
  (bind _tooltip_list (`local.Tooltip List`))
  (bind (_iteminventory_ _itemname _itemdescription) (break `/Game/Inventory/S_Item` (`self.This Item`)))
  (`KismetArrayLibrary.Array_Add` _tooltip_list "<Title>")
  (`KismetArrayLibrary.Array_Add` _tooltip_list (`KismetTextLibrary.Conv_TextToString` _itemname))
  (`KismetArrayLibrary.Array_Add` _tooltip_list "</> \n<Description>")
  (`KismetArrayLibrary.Array_Add` _tooltip_list (`KismetTextLibrary.Conv_TextToString` _itemdescription))
  (`KismetArrayLibrary.Array_Add` _tooltip_list "</>")
  (return (make `TooltipData` (`KismetStringLibrary.JoinStringArray` (`local.Tooltip List`)))))

(fn `UserConstructionScript`)