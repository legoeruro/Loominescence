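; Potion-crafting material actor whose tooltip presents it as a spawn box that spawns a box of its elemental type when pressed.
; GetTooltipData returns the result of GetTooltipDataFunc, which joins rich-text title and description fragments with the ItemElementalType name into tooltip data.
; The event graph and construction script are empty, so no spawning logic lives in this Blueprint.
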(fn `GetTooltipData`
  (returns (ReturnValue :type "TooltipData Structure"))
  (return (`self.GetTooltipDataFunc`)))

(fn `GetTooltipDataFunc`
  (returns (ReturnValue :type "TooltipData Structure"))
  (locals (`Tooltip list` :type "Array of String"))
  (bind _tooltip_list (`local.Tooltip list`))
  (bind _tooltip_list_2 (`local.Tooltip list`))
  (bind _tooltip_list_3 (`local.Tooltip list`))
  (`KismetArrayLibrary.Array_Add` _tooltip_list_3 "<Title>Spawn box  </> ")
  (`KismetArrayLibrary.Array_Add` _tooltip_list_3 " \n")
  (`KismetArrayLibrary.Array_Add` _tooltip_list_2 "<Description> Pressing on it spawns ")
  (`KismetArrayLibrary.Array_Add` _tooltip_list_2 "a box of type ")
  (`KismetArrayLibrary.Array_Add` _tooltip_list (`|GetEnumeratorNameAsString` (`self.ItemElementalType`)))
  (`KismetArrayLibrary.Array_Add` _tooltip_list "</>")
  (return (make `TooltipData` (`KismetStringLibrary.JoinStringArray` _tooltip_list ""))))

(fn `UserConstructionScript`)