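; BP_Poe is an actor that follows the player pawn, hovering above it.
; On BeginPlay it casts player pawn 0 to BP_PlayerBase and caches the reference.
; Each tick, while that reference is valid, it interpolates its location toward a fixed height offset above the player with VInterpTo for a smooth trailing motion, and snaps its rotation to match the player's.
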(event `self.ReceiveBeginPlay`
  (bind _asbp_player_base (cast `/Game/Blueprints/Player/BP_PlayerBase` (`GameplayStatics.GetPlayerPawn` 0)))
  (set `self.As BP Player Base` _asbp_player_base))

(event `self.ReceiveTick`
  (params (DeltaSeconds :type "Float (single-precision)"))
  (bind (_returnvalue_location _returnvalue_rotation) (`KismetMathLibrary.BreakTransform` (`self.GetTransform` (`self.As BP Player Base`))))
  (`/Engine/EditorBlueprintResources/StandardMacros.IsValid` (`self.As BP Player Base`)
    (:`Is Valid`
      (`self.K2_SetActorLocation` (`KismetMathLibrary.VInterpTo` (`self.K2_GetActorLocation`) (+ _returnvalue_location (0.0 0.0 100.0)) DeltaSeconds 5.0))
      (`self.K2_SetActorRotation` _returnvalue_rotation))))

(fn `UserConstructionScript`)