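; BP_PotionProjectile is a thrown potion whose effect depends on its PotionType.
; On hitting a BP_SmallMob1, it deals damage, plays a shatter sound, triggers the matching mob effect, then bursts in potion-colored Niagara.
; Explosion potions destroy BP_DestructableFloor with an explosion effect; other types ignore it, and any other hit simply breaks the bottle.
; BeginPlay waits briefly, then spawns an emitter and unhides the bottle.
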(event `OnDestroy`
  (bind (_returnvalue_location _returnvalue_rotation) (`KismetMathLibrary.BreakTransform` (`self.GetTransform`)))
  (bind _returnvalue (`NiagaraFunctionLibrary.SpawnSystemAtLocation` "/Game/Assets/ParticalEffect/NS_PotionBreak.NS_PotionBreak" _returnvalue_location _returnvalue_rotation))
  (`NiagaraComponent.SetVariableLinearColor` _returnvalue "PotionColor" (`self.PotionColor`))
  (`self.K2_DestroyActor`))

(event `self.ReceiveBeginPlay`
  (`KismetSystemLibrary.Delay` 5.0)
  (`GameplayStatics.SpawnEmitterAtLocation` null (`self.K2_GetActorLocation`))
  (`SceneComponent.SetHiddenInGame` (`self.Bottle`) false false))

(event `self.Sphere.OnComponentHit`
  (params (HitComponent :type "PrimitiveComponent Object Reference") (OtherActor :type "Actor Object Reference") (OtherComp :type "PrimitiveComponent Object Reference") (NormalImpulse :type "Vector Structure") (Hit :type "HitResult Structure (by ref)"))
  (bind (_returnvalue_location _returnvalue_rotation) (`KismetMathLibrary.BreakTransform` (`self.GetTransform`)))
  (bind _asbp_small_mob_1 (cast `/Game/Blueprints/Enemies/BP_SmallMob1` OtherActor)
    (:`then`
      (`GameplayStatics.ApplyDamage` _asbp_small_mob_1 10.0)
      (`GameplayStatics.PlaySound2D` "/Game/Assets/SFX/Glass_Shatter_1.Glass_Shatter_1" 1.0 1.0 0.0 null null)
      (switch `string` (`self.PotionType`)
        (:`Float`
          (`/Game/Blueprints/Enemies/BP_SmallMob1.FloatUp` _asbp_small_mob_1)
          (`self.OnDestroy`))
        (:`DoubleJump`
          (`/Game/Blueprints/Enemies/BP_SmallMob1.DoubleAttack` _asbp_small_mob_1)
          (`self.OnDestroy`))
        (:`Explosion`
          (`/Game/Blueprints/Enemies/BP_SmallMob1.Explode` _asbp_small_mob_1)
          (`self.OnDestroy`))
        (:`Speed`
          (`/Game/Blueprints/Enemies/BP_SmallMob1.Increase Speed` _asbp_small_mob_1)
          (`self.OnDestroy`))
        (:`Heal`
          (`/Game/Blueprints/Enemies/BP_SmallMob1.Heal` _asbp_small_mob_1)
          (`self.OnDestroy`))))
    (:`CastFailed`
      (bind _asbp_destructable_floor (cast `/Game/Blueprints/BP_DestructableFloor` OtherActor)
        (:`then`
          (if (== (`self.PotionType`) "Explosion")
            (`NiagaraFunctionLibrary.SpawnSystemAtLocation` "/Game/Assets/ParticalEffect/NS_Explosion.NS_Explosion" _returnvalue_location _returnvalue_rotation)
            (`self.K2_DestroyActor` _asbp_destructable_floor)
            (`self.K2_DestroyActor`)))
        (:`CastFailed`
          (`self.OnDestroy`))))))

(fn `UserConstructionScript`)