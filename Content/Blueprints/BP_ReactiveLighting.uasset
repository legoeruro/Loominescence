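; BP_ReactiveLighting is a point light that changes intensity when the player enters or leaves its sphere.
; BeginPlay applies the inactive intensity, color and falloff settings to the light.
; Player overlap plays the LightFade timeline to lerp intensity from inactive toward active.
; End overlap reverses a separate timeline, Timeline, rather than LightFade, driving the same lerp from its own Intensity track.
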(event `self.ReceiveBeginPlay`
  (bind _pointlight (`self.PointLight`))
  (`LightComponent.SetIntensity` _pointlight (`self.InactiveIntensity`))
  (`LightComponent.SetLightColor` _pointlight (`self.Color`) true)
  (`PointLightComponent.SetLightFalloffExponent` (`self.PointLight`) (`self.LightFalloff`))
  (`PointLightComponent.SetUseInverseSquaredFalloff` (`self.PointLight`) (`self.InverseSquareFalloff`)))

(event `self.Sphere.OnComponentBeginOverlap`
  (params (OverlappedComponent :type "PrimitiveComponent Object Reference") (OtherActor :type "Actor Object Reference") (OtherComp :type "PrimitiveComponent Object Reference") (OtherBodyIndex :type Integer) (bFromSweep :type Boolean) (SweepResult :type "HitResult Structure (by ref)"))
  (cast `/Game/Blueprints/Player/BP_PlayerBase` OtherActor)
  (bind (_direction _intensity) (`Timeline|LightFade`)
    (:`Update`
      (`LightComponent.SetIntensity` (`self.PointLight`) (`KismetMathLibrary.Lerp` (`self.InactiveIntensity`) (`self.ActiveIntensity`) _intensity)))))

(event `self.Sphere.OnComponentEndOverlap`
  (params (OverlappedComponent :type "PrimitiveComponent Object Reference") (OtherActor :type "Actor Object Reference") (OtherComp :type "PrimitiveComponent Object Reference") (OtherBodyIndex :type Integer))
  (cast `/Game/Blueprints/Player/BP_PlayerBase` OtherActor)
  (bind (_direction _intensity) (`Timeline|Timeline` :!via `Reverse`)
    (:`Update`
      (`LightComponent.SetIntensity` (`self.PointLight`) (`KismetMathLibrary.Lerp` (`self.InactiveIntensity`) (`self.ActiveIntensity`) _intensity)))))

(fn `UserConstructionScript`)