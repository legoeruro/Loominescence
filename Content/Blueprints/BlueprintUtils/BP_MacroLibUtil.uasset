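; Utility macro library that builds item tooltip data from an item struct.
; GetItemTooltipDataFromItemStruct wraps the item name in Title markup tags and the description in Description tags, in the style of rich text.
; It collects these pieces in a string list, joins them without a separator and returns the result as tooltip data.
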(fn `GetItemTooltipDataFromItemStruct`
  (params (`Item Struct` :type "/Game/Inventory/S_Item Structure"))
  (returns (ReturnValue :type "TooltipData Structure"))
  (locals (`Tooltip List` :type "Array of String"))
  (bind (_iteminventory_ _itemname _itemdescription) (break `/Game/Inventory/S_Item` `Item Struct`))
  (bind _tooltip_list (`local.Tooltip List`))
  (`KismetArrayLibrary.Array_Add` _tooltip_list "<Title>")
  (`KismetArrayLibrary.Array_Add` _tooltip_list (`KismetTextLibrary.Conv_TextToString` _itemname))
  (`KismetArrayLibrary.Array_Add` _tooltip_list "</> \n<Description>")
  (`KismetArrayLibrary.Array_Add` _tooltip_list (`KismetTextLibrary.Conv_TextToString` _itemdescription))
  (`KismetArrayLibrary.Array_Add` _tooltip_list "</>")
  (return (make `TooltipData` (`KismetStringLibrary.JoinStringArray` (`local.Tooltip List`)))))