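; BP_ResourceSpanwer is a spawner actor that places an inventory resource item in the world and can respawn it later.
; On begin play it spawns the configured ItemClass at its own transform, always spawning, and sets itself as the Spawner on the resulting BP_BASEItem.
; RequestRespawn stores a given transform and schedules the same spawn event on a one-minute timer.
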(event `self.ReceiveBeginPlay`
  (set `self.SpawnTransform` (`self.GetTransform`))
  (`self.Spawn Resource`))

(event `Request Respawn`
  (params (Transform :type "Transform Structure"))
  (set `self.SpawnTransform` Transform)
  (`KismetSystemLibrary.K2_SetTimerDelegate` (delegate `Spawn Resource`) 60.0))

(event `Spawn Resource`
  (bind (_spawntransform_location _spawntransform_rotation) (`KismetMathLibrary.BreakTransform` (`self.SpawnTransform`)))
  (bind _returnvalue (`|SpawnActorFromClass` (`self.ItemClass`) (`KismetMathLibrary.MakeTransform` _spawntransform_location _spawntransform_rotation) "AlwaysSpawn" "MultiplyWithRoot" null null))
  (bind _asbp_baseitem (cast `/Game/Inventory/BP_BASEItem` _returnvalue))
  (set `/Game/Inventory/BP_BASEItem.Spawner` self _asbp_baseitem))

(fn `UserConstructionScript`)