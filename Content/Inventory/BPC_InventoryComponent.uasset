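; Inventory component that stores picked-up items in a fixed-size array and opens the WBP_InventoryGrid widget on IA_Inventory.
; It loads items from BP_GameInstance's PersistentInventoryItems on BeginPlay and writes them back after adds and deletions.
; AddToInventory stacks matching items up to the slot limit or fills a free slot, then destroys the actor.
; Deletion leaves a blank placeholder for reuse, changes refresh the grid, and IsElementInInventory checks for an elemental type.
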(event `self.ReceiveBeginPlay`
  ; Begin Play
  (bind _returnvalue (`|CreateWidget` "/Game/Inventory/WBP_InventoryGrid.WBP_InventoryGrid_C"))
  (set `self.InventoryGridRef` _returnvalue)
  (bind _items (`self.Get Global Items List`))
  (bind _output_get (set `self.Items` _items))
  (`KismetArrayLibrary.Array_Resize` _output_get (`self.InventorySize`))
  (`/Game/Inventory/WBP_InventoryGrid.Refresh Inventory` (`self.InventoryGridRef`) self))

(event `EnhancedInput|/Game/InputAction/IA_Inventory`
  (params (ActionValue :type Boolean) (ElapsedSeconds :type "Float (double-precision)") (TriggeredSeconds :type "Float (double-precision)") (InputAction :type "InputAction Object Reference" :default "/Game/InputAction/IA_Inventory.IA_Inventory"))
  (bind _returnvalue (`GameplayStatics.GetPlayerController` 0))
  (bind _inventorygridref (`self.InventoryGridRef`))
  (bind _inventorygridref_2 (`self.InventoryGridRef`))
  ; Inventory Action
  (:`Triggered`
    (if (not (`Widget.IsInViewport` _inventorygridref))
      (`UserWidget.AddToViewport` _inventorygridref 0)
      (set `PlayerController.bShowMouseCursor` true _returnvalue)
      (`WidgetBlueprintLibrary.SetInputMode_UIOnlyEx` _returnvalue _inventorygridref_2)
      (set `UserWidget.bIsFocusable` true _inventorygridref_2))))

(fn `Add to Inventory`
  (params (ItemActor :type "/Game/Inventory/BP_BASEItem Object Reference"))
  (locals (Local_Item_Interacted :type "/Game/Inventory/BP_BASEItem Object Reference"))
  (bind _items (`self.Items`))
  (bind _items_2 (`self.Items`))
  (bind _firstemptyindex (`self.FirstEmptyIndex`))
  (bind _currentindex (`self.CurrentIndex`))
  (bind (_iteminventory_ _itemname _itemdescription _itemstackable_ _itemamount _itemmesh _itemimage _itemhealable_ _itemhealamount) (break `/Game/Inventory/S_Item` (`/Game/Inventory/BP_BASEItem.Item` (`local.Local_Item_Interacted`))))
  (set `local.Local_Item_Interacted` ItemActor)
  (for (_array_element _array_index) (`self.Items`)
    (`/Engine/EditorBlueprintResources/StandardMacros.IsValid` (`local.ItemActor`)
      (:`Is Valid`
        (set `self.CurrentIndex` _array_index)
        (bind (_can_add_ _new_item_amount) (`self.Should Stack Items?` _array_element (`/Game/Inventory/BP_BASEItem.Item` (`local.Local_Item_Interacted`))))
        (if _can_add_
          ; Stack Item
          (set `self.NewItemAmount` _new_item_amount)
          (`KismetArrayLibrary.Array_Set` (`self.Items`) (`self.CurrentIndex`) (make `/Game/Inventory/S_Item` _iteminventory_ _itemname _itemdescription _itemstackable_ (`self.NewItemAmount`) _itemmesh _itemimage _itemhealable_ _itemhealamount "None" false null))
          (`/Game/Inventory/WBP_InventoryGrid.Refresh Inventory` (`self.InventoryGridRef`) self :!label _label)
          (`Actor.K2_DestroyActor` (`local.Local_Item_Interacted`))
          (`KismetSystemLibrary.PrintString` "Item Added into Inventory." false)
          (`self.Update Global Items List as Local List`)
          (`self.InventoryChanged`)
          (return)
          (else
            ; First Time Picking up a Stackable Item, or Picking up a Nonstackable Item
            (bind _has_space_ (`self.Space in Inventory?` _new_item_amount))
            (if _has_space_
              (set `self.FirstEmptyIndex` -1)
              ; Loop through Item list and find Fake empty slot
              (for (_array_element_2 _array_index_2) _items_2
                (if (and (not (`.ItemInventory?_27_594ED0DB4451C5735DBE22BCF4DA66BB` (break `/Game/Inventory/S_Item` _array_element_2))) (== (`self.FirstEmptyIndex`) -1))
                  (set `self.FirstEmptyIndex` _array_index_2)))
              ; If find no Fake empty slot due to Deletion, Add to Inventory normally. If there is a Fake empty slot, add new Item into that Index instead.
              (if (== _firstemptyindex -1)
                (`KismetArrayLibrary.Array_Insert` _items (`/Game/Inventory/BP_BASEItem.Item` (`local.Local_Item_Interacted`)) _currentindex)
                (`KismetArrayLibrary.Array_Remove` _items (- (`self.InventorySize`) _currentindex))
                (goto _label)
                (else
                  (`KismetArrayLibrary.Array_Set` _items_2 _firstemptyindex (`/Game/Inventory/BP_BASEItem.Item` (`local.Local_Item_Interacted`)))
                  (goto _label))))))))))

(fn `DeleteItemAtIndex`
  (params (Index :type Integer))
  (`KismetArrayLibrary.Array_Set` (`self.Items`) Index (make `/Game/Inventory/S_Item` false "" "" false 0 null null false 0 "None" false null))
  (`self.InventoryChanged`)
  (`/Game/Inventory/WBP_InventoryGrid.Refresh Inventory` (`self.InventoryGridRef`) self)
  (`self.Update Global Items List as Local List`))

(fn `Get Global Items List`
  (returns (Items :type "Array of /Game/Inventory/S_Item Structure"))
  (bind _asbp_game_instance (cast `/Game/BP_GameInstance` (`GameplayStatics.GetGameInstance`)))
  (return (`/Game/BP_GameInstance.PersistentInventoryItems` _asbp_game_instance)))

(fn `GetItems`
  (returns (ReturnValue :type "Array of /Game/Inventory/S_Item Structure"))
  (bind _items (`self.Get Global Items List`))
  (return _items))

(fn `IsElementInInventory`
  (params (`Elemental Type` :type "EElementalType Enum" :default "None"))
  (returns (IsInArray :type Boolean))
  (bind _items (`self.Items`))
  (`KismetSystemLibrary.PrintString` "Hello")
  (`KismetSystemLibrary.PrintString` (`|GetEnumeratorNameAsString` `Elemental Type`))
  (`KismetSystemLibrary.PrintString` (`KismetStringLibrary.Conv_IntToString` (`KismetArrayLibrary.Array_Length` _items)))
  (for _array_element _items
    (bind (_iteminventory_ _itemname _itemdescription _itemstackable_ _itemamount _itemmesh _itemimage _itemhealable_ _itemhealamount _itemelement) (break `/Game/Inventory/S_Item` _array_element))
    (`KismetSystemLibrary.PrintString` (`|GetEnumeratorNameAsString` _itemelement))
    (if (== (`KismetMathLibrary.Conv_ByteToInt` `Elemental Type`) (`KismetMathLibrary.Conv_ByteToInt` _itemelement))
      (return true)))
  (return false))

(fn `Should Stack Items?`
  (params (`Item From Inventory` :type "/Game/Inventory/S_Item Structure") (`Item From Current Actor` :type "/Game/Inventory/S_Item Structure"))
  (returns (`Can Add?` :type Boolean) (`New Item Amount` :type Integer))
  (bind (_iteminventory_ _itemname _itemdescription _itemstackable_ _itemamount) (break `/Game/Inventory/S_Item` `Item From Inventory`))
  (bind (_iteminventory__2 _itemname_2 _itemdescription_2 _itemstackable__2 _itemamount_2) (break `/Game/Inventory/S_Item` `Item From Current Actor`))
  (bind _returnvalue (+ _itemamount _itemamount_2))
  (if (and (<= _returnvalue (`self.InventorySlotSize`)) (`KismetTextLibrary.EqualEqual_TextText` _itemname _itemname_2) _iteminventory__2 _itemstackable__2)
    (return true _returnvalue)
    (else
      (return false _itemamount))))

(fn `Space in Inventory?`
  (params (`Item Amount From Inventory` :type Integer))
  (returns (`Has Space?` :type Boolean))
  (if (== `Item Amount From Inventory` 0)
    (return true)
    (else
      (return false))))

(fn `Update Global Items List as Local List`
  (bind _asbp_game_instance (cast `/Game/BP_GameInstance` (`GameplayStatics.GetGameInstance`)))
  (set `/Game/BP_GameInstance.PersistentInventoryItems` (`self.Items`) _asbp_game_instance)
  (return))